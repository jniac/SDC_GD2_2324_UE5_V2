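; BP_stairs_IMA is an actor with five box steps that rise into a staircase while something overlaps it and lower when the overlap ends.
; Overlap begin and end play or reverse a timeline that drives an Opening value.
; Every tick, Updatestairs sets each box's relative Z to a lerp between compact and open spacing multiplied by its index, so the first step stays at zero height.
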(event EventBeginPlay)

(event Collision|EventActorEndOverlap
  (params (OtherActor :type Actor%20Object%20Reference))
  (bind _opening (Timeline|Timeline Reverse)
    (:Update
      (Variables|Default|Setopening _opening))))

(event EventTick
  (params (DeltaSeconds :type Float%20%28single-precision%29))
  (CallFunction|Updatestairs))

(event Collision|EventActorBeginOverlap
  (params (OtherActor :type Actor%20Object%20Reference))
  (bind _opening (Timeline|Timeline Play)
    (:Update
      (Variables|Default|Setopening _opening))))

(fn ConstructionScript)

(fn Updatestairs
  (for (_array_element _array_index) (Utilities|Array|MakeArray (Variables|Default|GetIMA_SM_Box) (Variables|Default|GetIMA_SM_Box1) (Variables|Default|GetIMA_SM_Box2) (Variables|Default|GetIMA_SM_Box3) (Variables|Default|GetIMA_SM_Box4))
    (Transformation|SetRelativeLocation _array_element (Math|Vector|MakeVector 0.0 0.0 (* (Math|Float|Lerp 2.0 25.0 (Variables|Default|Getopening)) (Math|Conversions|ToFloat(Integer) _array_index))) false false)))